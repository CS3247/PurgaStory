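; Test actor for a possess mechanic, with a static mesh that reacts to attach, detach and highlight events.
; AttachPossess switches the mesh to the IgnoreOnlyPawn collision profile, and DetachPossess switches it to BlockAll.
; Highlight sets material slot 0 with no material specified, while Tick reapplies DefaultMaterial every frame, so any highlight must be re-triggered continuously to persist.
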(event Custom|AttachPossess
  (Collision|SetCollisionProfileName (Variables|Default|GetStaticMesh) "IgnoreOnlyPawn" :!class /Script/Engine.PrimitiveComponent))

(event Custom|DetachPossess
  (Collision|SetCollisionProfileName (Variables|Default|GetStaticMesh) "BlockAll" :!class /Script/Engine.PrimitiveComponent))

(event Custom|Highlight
  (Rendering|Material|SetMaterial (Variables|Default|GetStaticMesh) 0 0))

(event Collision|EventActorBeginOverlap
  (params (OtherActor :type Actor%20Object%20Reference)))

(event EventTick
  (params (DeltaSeconds :type Float%20%28single-precision%29))
  (Rendering|Material|SetMaterial (Variables|Default|GetStaticMesh) 0 (Variables|Default|GetDefaultMaterial)))

(fn ConstructionScript)