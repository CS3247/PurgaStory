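; Player character for a possession mechanic: clicking an aimed actor tagged canPossess swaps the character into that object.
; Tick traces from the camera to place an aim billboard and highlight candidates via messages.
; Possessing detaches the old object, teleports to and attaches the new one, then sets run or jump speeds from its tags.
; Also handles movement, zoom, camera fades, and R to reload the StationaryCameras level.
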(event Collision|EventActorBeginOverlap
  (params (OtherActor :type Actor%20Object%20Reference)))

(event EventTick
  (params (DeltaSeconds :type Float%20%28single-precision%29))
  (bind _materialbillboard (Variables|Default|GetMaterialBillboard))
  (bind _camera (Variables|Default|GetCamera))
  (bind _returnvalue (Transformation|GetWorldLocation _camera))
  (bind _returnvalue_2 (Math|Vector|GetForwardVector _camera))
  (bind _returnvalue_3 (* _returnvalue_2 4.5e+02))
  (bind _returnvalue_4 (+ _returnvalue _returnvalue_3))
  ;[1 1 1] Aimming
  (bind (_outhit _returnvalue_5) (Collision|LineTraceByChannel _returnvalue _returnvalue_4 "TraceTypeQuery1" false (Utilities|Array|MakeArray (Variables|Default|GetCurrentPossess)) "None" true "(R=1.000000,G=0.000000,B=0.000000,A=1.000000)" "(R=0.000000,G=1.000000,B=0.000000,A=1.000000)" 0.1))
  (if _returnvalue_5
    (Transformation|SetWorldLocation _materialbillboard (.ImpactPoint (Collision|BreakHitResult _outhit)) false false)
    (if (Actor|ActorHasTag (.HitActor (Collision|BreakHitResult _outhit)) "canPossess")
      (if (not (== (Variables|Default|GetCurrentPossess) (.HitActor (Collision|BreakHitResult _outhit))))
        (Class|Object|Highlight(Message) (.HitActor (Collision|BreakHitResult _outhit)))))
    (else
      (Transformation|SetWorldLocation _materialbillboard _returnvalue_4 false false))))

(event EventBeginPlay
  (CameraFades|StartCameraFade :self (Game|GetPlayerCameraManager 0) :FromAlpha 1.0 :Duration 2.0))

(event Input|ActionEvents|InputActionJump
  (params (Key :type Key%20Structure :default "AnyKey"))
  ;[1 1 1] Controls
  (:Pressed
    (Character|Jump)
    (if (Actor|ActorHasTag (Variables|Default|GetCurrentPossess) "JumpImproved")
      (Audio|PlaySoundatLocation "/Game/Audio/SoundWaves/Effect/SW_Jump_1.SW_Jump_1" (Transformation|GetActorLocation))))
  (:Released
    (Character|StopJumping)))

(event Input|AxisEvents|InputAxisMoveForward
  (params (AxisValue :type Float%20%28single-precision%29))
  ;[1 1 1] Controls
  (Pawn|Input|AddMovementInput (Transformation|GetActorForwardVector) AxisValue false))

(event Input|AxisEvents|InputAxisLookUp
  (params (AxisValue :type Float%20%28single-precision%29))
  ;[1 1 1] Controls
  (Pawn|Input|AddControllerPitchInput AxisValue))

(event Input|AxisEvents|InputAxisZoomIn
  (params (AxisValue :type Float%20%28single-precision%29))
  ;[1 1 1] Controls
  (bind _output_get (Variables|Default|SetCameraArmLength (Math|Float|Clamp(Float) (+ (* AxisValue 2e+01) (Variables|Default|GetCameraArmLength)) 3e+01 2e+02)))
  (Variables|/Script/Engine.SpringArmComponent|SetTargetArmLength (Variables|Default|GetSpringArm) _output_get))

(event Input|AxisEvents|InputAxisMoveRight
  (params (AxisValue :type Float%20%28single-precision%29))
  ;[1 1 1] Controls
  (Pawn|Input|AddMovementInput (Transformation|GetActorRightVector) AxisValue false))

(event Input|AxisEvents|InputAxisTurn
  (params (AxisValue :type Float%20%28single-precision%29))
  ;[1 1 1] Controls
  (Pawn|Input|AddControllerYawInput AxisValue))

(event Input|MouseEvents|LeftMouseButton
  (params (Key :type Key%20Structure :default "AnyKey"))
  (bind _self self)
  (bind _charactermovement (Variables|Character|GetCharacterMovement))
  (bind _camera (Variables|Default|GetCamera))
  (bind _charactermovement_2 (Variables|Character|GetCharacterMovement))
  (bind _defaultjumpspeed (Variables|Default|GetDefaultJumpSpeed))
  (bind _returnvalue (Transformation|GetWorldLocation _camera))
  (bind _returnvalue_2 (Transformation|GetActorLocation _self))
  (:Pressed
    (bind (_outhit _returnvalue_3) (Collision|LineTraceByChannel _returnvalue (+ _returnvalue (* (Math|Vector|GetForwardVector _camera) 4.5e+02)) "TraceTypeQuery1" false (Utilities|Array|MakeArray (Variables|Default|GetCurrentPossess)) "None"))
    (if _returnvalue_3
      (if (Actor|ActorHasTag (.HitActor (Collision|BreakHitResult _outhit)) "canPossess")
        (Transformation|DetachFromActor (Variables|Default|GetCurrentPossess) "KeepWorld" "KeepWorld" "KeepRelative")
        (Class|Object|AttachPossess(Message) (.HitActor (Collision|BreakHitResult _outhit)))
        (Class|Object|DetachPossess(Message) (Variables|Default|GetCurrentPossess))
        (Variables|Default|SetCurrentPossess (.HitActor (Collision|BreakHitResult _outhit)))
        (Transformation|SetActorLocation (+ (Transformation|GetActorLocation (.HitActor (Collision|BreakHitResult _outhit))) (Math|Vector|MakeVector 0.0 0.0 (Variables|/Script/Engine.CapsuleComponent|GetCapsuleHalfHeight (Variables|Collision|GetCapsuleComponent)))) false false)
        (CameraFades|StartCameraFade (Game|GetPlayerCameraManager 0) 1.0 0.0 0.5 "(R=1.000000,G=1.000000,B=1.000000,A=1.000000)" false false)
        (Transformation|AttachActorToActor (.HitActor (Collision|BreakHitResult _outhit)) _self "None" "KeepWorld" "KeepWorld" "KeepWorld" true)
        (Effects|SpawnEmitteratLocation 0 _returnvalue_2)
        (Audio|PlaySoundatLocation "/Game/Audio/SoundWaves/Effect/SW_Shot_1.SW_Shot_1" _returnvalue_2)
        (if (Actor|ActorHasTag (Variables|Default|GetCurrentPossess) "JumpImproved")
          (Variables|/Script/Engine.CharacterMovementComponent|SetMaxWalkSpeed _charactermovement (Variables|Default|GetDefaultWalkSpeed))
          (Variables|/Script/Engine.CharacterMovementComponent|SetJumpZVelocity _charactermovement (Variables|Default|GetImprovedJumpSpeed))
          (elif (Actor|ActorHasTag (Variables|Default|GetCurrentPossess) "RunImproved")
            (Variables|/Script/Engine.CharacterMovementComponent|SetMaxWalkSpeed _charactermovement_2 (Variables|Default|GetImprovedWalkSpeed))
            (Variables|/Script/Engine.CharacterMovementComponent|SetJumpZVelocity _charactermovement_2 _defaultjumpspeed)
            (else
              (Variables|/Script/Engine.CharacterMovementComponent|SetMaxWalkSpeed _charactermovement_2 (Variables|Default|GetDefaultWalkSpeed))
              (Variables|/Script/Engine.CharacterMovementComponent|SetJumpZVelocity _charactermovement_2 _defaultjumpspeed))))))))

(event Input|KeyboardEvents|R
  (params (Key :type Key%20Structure :default "AnyKey"))
  (:Pressed
    (CameraFades|StartCameraFade :self (Game|GetPlayerCameraManager 0) :ToAlpha 1.0 :Duration 0.5 :bHoldWhenFinished true)
    (Utilities|FlowControl|Delay 0.5)
    (Game|OpenLevel(byName) "StationaryCameras")))

(fn ConstructionScript)